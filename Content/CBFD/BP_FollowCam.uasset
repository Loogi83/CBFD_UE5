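; BP_FollowCam is a camera actor that trails the BP_Conker actor in the world.
; It finds and stores Conker on BeginPlay, then rotates its camera every tick to look at him.
; When Conker is farther away than Radius, the actor eases toward his location with a slow VInterpTo, without sweeping for collision.
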(event `self.ReceiveBeginPlay`
  (bind _returnvalue (`GameplayStatics.GetActorOfClass` "/Game/CBFD/Characters/Conker/BP_Conker.BP_Conker_C"))
  (set `self.Conker` _returnvalue))

(event `self.ReceiveTick`
  (params (DeltaSeconds :type "Float (single-precision)"))
  (bind _returnvalue (`self.K2_GetActorLocation` (`self.Conker`)))
  (`SceneComponent.K2_SetWorldRotation` (`self.Camera`) (`KismetMathLibrary.FindLookAtRotation` (`SceneComponent.K2_GetComponentLocation` (`self.Camera`)) _returnvalue) false false)
  (if (> (`KismetMathLibrary.Vector_Distance` (`self.K2_GetActorLocation`) _returnvalue) (`self.Radius`))
    (`self.K2_SetActorLocation` (`KismetMathLibrary.VInterpTo` (`self.K2_GetActorLocation`) (`self.K2_GetActorLocation` (`self.Conker`)) (`GameplayStatics.GetWorldDeltaSeconds`) 0.5))))

(fn `UserConstructionScript`)