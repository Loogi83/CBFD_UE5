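; Player Blueprint for Conker that is an input scaffold, with debug prints standing in for movement, jump and hover.
; On BeginPlay it adds the IMC_Conker mapping context to the Enhanced Input local player subsystem.
; IA_Movement prints its X and Y axis values, while IA_Hover prints a jump message on Started and hover status on Triggered, Canceled and Completed.
; No actual movement logic is implemented.
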(event `self.ReceiveBeginPlay`
  (`EnhancedInputSubsystemInterface.AddMappingContext` (subsystem `EnhancedInputLocalPlayerSubsystem`) "/Game/CBFD/Characters/Conker/Inputs/IMC_Conker.IMC_Conker" 0 (struct)))

(event `EnhancedInput|/Game/CBFD/Characters/Conker/Inputs/IA_Movement`
  (params (ActionValue :type "Vector2D Structure") (ElapsedSeconds :type "Float (double-precision)") (TriggeredSeconds :type "Float (double-precision)") (InputAction :type "InputAction Object Reference" :default "/Game/CBFD/Characters/Conker/Inputs/IA_Movement.IA_Movement"))
  (:`Triggered`
    (`KismetSystemLibrary.PrintString` (`KismetTextLibrary.Conv_TextToString` (`|FormatText` "X Axis = {X}, Y Axis = {Y}" ActionValue_X ActionValue_Y)))))

(event `EnhancedInput|/Game/CBFD/Characters/Conker/Inputs/IA_Hover`
  (params (ActionValue :type Boolean) (ElapsedSeconds :type "Float (double-precision)") (TriggeredSeconds :type "Float (double-precision)") (InputAction :type "InputAction Object Reference" :default "/Game/CBFD/Characters/Conker/Inputs/IA_Hover.IA_Hover"))
  (:`Triggered`
    (`KismetSystemLibrary.PrintString` "Hovering"))
  (:`Started`
    (`KismetSystemLibrary.PrintString` "Jump"))
  (:`Canceled`
    (`KismetSystemLibrary.PrintString` "Hover Stopped"))
  (:`Completed`
    (`KismetSystemLibrary.PrintString` "Hover Completed")))

(fn `UserConstructionScript`)