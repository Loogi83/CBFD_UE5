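; Conker's player character Blueprint, handling Enhanced Input movement, camera, crouch, jump and hover.
; Jumping from a crouch launches higher, and pressing jump while falling triggers a one-use, low-gravity hover ended by timer or release.
; A looping floor check re-arms hover after landing.
; A timer-driven auto-camera eases control rotation toward CameraDirection, while manual camera input cancels it and starts a delay timer.
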(event `EnhancedInput|/Game/CBFD/Characters/Conker/Inputs/IA_Crouch`
  (params (ActionValue :type Boolean) (ElapsedSeconds :type "Float (double-precision)") (TriggeredSeconds :type "Float (double-precision)") (InputAction :type "InputAction Object Reference" :default "/Game/CBFD/Characters/Conker/Inputs/IA_Crouch.IA_Crouch"))
  ;[1 1 1] Crouch
  (:`Started`
    (`self.Crouch`))
  (:`Completed`
    (`self.UnCrouch`)))

(event `EnhancedInput|/Game/CBFD/Characters/Conker/Inputs/IA_Jump`
  (params (ActionValue :type Boolean) (ElapsedSeconds :type "Float (double-precision)") (TriggeredSeconds :type "Float (double-precision)") (InputAction :type "InputAction Object Reference" :default "/Game/CBFD/Characters/Conker/Inputs/IA_Jump.IA_Jump"))
  (bind _charactermovement (`self.CharacterMovement`))
  ;[1 1 1] Jump/Hover
  (:`Started`
    (switch `EMovementMode` (`CharacterMovementComponent.MovementMode` (`self.CharacterMovement`))
      (:`MOVE_Walking`
        ;;[1 1 1] Crouch Jump
        (set `CharacterMovementComponent.JumpZVelocity` (`KismetMathLibrary.SelectFloat` 1000.0 500.0 (`NavMovementComponent.IsCrouching` _charactermovement)) _charactermovement)
        (`self.UnCrouch`)
        (`KismetSystemLibrary.Delay` 0.01)
        (`self.Jump`))
      (:`MOVE_Falling`
        (if (`self.canHover`)
          (`self.Hover`)))))
  (:`Canceled`
    (`self.StopJumping`))
  (:`Completed`
    (if (`KismetSystemLibrary.K2_IsValidTimerHandle` (`self.HoverTimer`))
      (`KismetSystemLibrary.K2_ClearAndInvalidateTimerHandle` (`self.HoverTimer`))
      (`self.StopHover`))))

(event `self.ReceivePossessed`
  (params (NewController :type "Controller Object Reference"))
  ;[1 1 1] On Possess
  (bind _asplayer_controller (cast `PlayerController` NewController))
  (bind _output_get (set `self.PlayerController` _asplayer_controller))
  (bind _returnvalue (pcsubsystem `EnhancedInputLocalPlayerSubsystem` _output_get))
  (`/Engine/EditorBlueprintResources/StandardMacros.IsValid` _returnvalue
    (:`Is Valid`
      (`EnhancedInputSubsystemInterface.AddMappingContext` _returnvalue "/Game/CBFD/Characters/Conker/Inputs/IMC_Conker.IMC_Conker" 0 (struct))
      (`self.CameraFollow`))))

(event `EnhancedInput|/Game/CBFD/Characters/Conker/Inputs/IA_Movement`
  (params (ActionValue :type "Vector2D Structure") (ElapsedSeconds :type "Float (double-precision)") (TriggeredSeconds :type "Float (double-precision)") (InputAction :type "InputAction Object Reference" :default "/Game/CBFD/Characters/Conker/Inputs/IA_Movement.IA_Movement"))
  (bind (_returnvalue_roll _returnvalue_pitch _returnvalue_yaw) (`KismetMathLibrary.BreakRotator` (`self.GetControlRotation`)))
  (bind (_returnvalue_roll_2 _returnvalue_pitch_2 _returnvalue_yaw_2) (`KismetMathLibrary.BreakRotator` (`self.GetControlRotation`)))
  ;[1 1 1] Movement
  (:`Triggered`
    (`self.AddMovementInput` (`KismetMathLibrary.GetRightVector` (`KismetMathLibrary.MakeRotator` _returnvalue_roll_2 0.0 _returnvalue_yaw_2)) ActionValue_X)
    (`self.AddMovementInput` (`KismetMathLibrary.GetForwardVector` (`KismetMathLibrary.MakeRotator` 0.0 0.0 _returnvalue_yaw)) ActionValue_Y)))

(event `Hover`
  ;[1 1 1] Hover/Stop Hover
  (set `self.canHover` false)
  (bind _returnvalue (`KismetSystemLibrary.K2_SetTimerDelegate` (delegate `StopHover`) 1.5))
  (set `self.HoverTimer` _returnvalue)
  (`KismetSystemLibrary.Delay` 0.1)
  (set `CharacterMovementComponent.GravityScale` 0.2 (`self.CharacterMovement`))
  (bind _returnvalue_2 (`KismetSystemLibrary.K2_SetTimerDelegate` (delegate `FloorCheck`) 0.1 true))
  (set `self.FallingHandle` _returnvalue_2))

(event `StopHover`
  ;[1 1 1] Hover/Stop Hover
  (set `CharacterMovementComponent.GravityScale` 1.0 (`self.CharacterMovement`)))

(event `FloorCheck`
  ;[1 1 1] Hover/Stop Hover
  (if (not (`NavMovementComponent.IsFalling` (`self.CharacterMovement`)))
    (set `self.canHover` true)
    (`KismetSystemLibrary.K2_ClearAndInvalidateTimerHandle` (`self.FallingHandle`))))

(event `EnhancedInput|/Game/CBFD/Characters/Conker/Inputs/IA_Camera`
  (params (ActionValue :type "Vector2D Structure") (ElapsedSeconds :type "Float (double-precision)") (TriggeredSeconds :type "Float (double-precision)") (InputAction :type "InputAction Object Reference" :default "/Game/CBFD/Characters/Conker/Inputs/IA_Camera.IA_Camera"))
  ;[1 1 1] Camera
  (:`Triggered`
    (if (`KismetSystemLibrary.K2_IsValidTimerHandle` (`self.CameraFollowTimer`))
      (`KismetSystemLibrary.K2_ClearAndInvalidateTimerHandle` (`self.CameraFollowTimer`)))
    (`self.AddControllerPitchInput` (* ActionValue_Y -1.0))
    (`self.AddControllerYawInput` ActionValue_X)
    (`KismetSystemLibrary.K2_SetTimerDelegate` (`|CreateDelegate` :!event `CameraFollow`) 3.0)))

(event `CameraFollow`
  ;[1 1 1] Camera Follow
  (bind _returnvalue (`KismetSystemLibrary.K2_SetTimerDelegate` (delegate `Rotate`) 0.01 true))
  (set `self.CameraFollowTimer` _returnvalue))

(event `Rotate`
  ;[1 1 1] Camera Follow
  (`Controller.SetControlRotation` (`self.PlayerController`) (`KismetMathLibrary.RInterpTo` (`Controller.GetControlRotation` (`self.PlayerController`)) (`SceneComponent.K2_GetComponentRotation` (`self.CameraDirection`)) (`GameplayStatics.GetWorldDeltaSeconds`) (`self.CameraAutoSpeed`))))

(fn `UserConstructionScript`)